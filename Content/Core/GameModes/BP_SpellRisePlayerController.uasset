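; SpellRise player controller that sets up local input, the player HUD, the pause menu and cursor modes.
; On BeginPlay, the local controller adds default and mouse-look Enhanced Input contexts, enters game-only input and creates W_PlayerHUD unless the pause menu is showing.
; Escape opens WB_PauseMenu if not already displayed, switching to game-and-UI input with a visible cursor.
; Z flip-flops between that cursor mode and game-only input.
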(event `self.ReceiveBeginPlay`
  (if (`self.IsLocalPlayerController`)
    (`EnhancedInputSubsystemInterface.AddMappingContext` (subsystem `EnhancedInputLocalPlayerSubsystem`) "/Game/Input/IMC_MouseLook.IMC_MouseLook" 0 (struct))
    (`EnhancedInputSubsystemInterface.AddMappingContext` (subsystem `EnhancedInputLocalPlayerSubsystem`) "/Game/Input/IMC_Default.IMC_Default" 0 (struct))
    (`WidgetBlueprintLibrary.SetInputMode_GameOnly` self)
    (set `self.bShowMouseCursor` false)
    (bind _wb_pausemenu (`self.WB_PauseMenu`)
      (:`then`
        (if (not (`Widget.IsInViewport` _wb_pausemenu))
          (bind _returnvalue (`|CreateWidget` "/Game/UI/Widgets/W_PlayerHUD.W_PlayerHUD_C" self :!label _label))
          (`UserWidget.AddToViewport` _returnvalue 0)))
      (:`else`
        (goto _label)))))

(event `Key|Escape`
  (params (Key :type "Key Structure"))
  ;[0.05098 0.05098 0.05098] Open Pause Menu
  (:`Pressed`
    (bind _wb_pausemenu (`self.WB_PauseMenu`)
      (:`then`
        (if (not (`Widget.IsInViewport` _wb_pausemenu))
          (bind _returnvalue (`|CreateWidget` "/Game/UI/Widgets/PauseMenu/WB_PauseMenu.WB_PauseMenu_C" self :!label _label_2))
          (bind _output_get (set `self.WB_PauseMenu` _returnvalue))
          (`UserWidget.AddToViewport` _output_get 0)
          (`WidgetBlueprintLibrary.SetInputMode_GameAndUIEx` self (`self.WB_PauseMenu`))
          (set `self.bShowMouseCursor` true)))
      (:`else`
        (goto _label_2)))))

(event `Key|Z`
  (params (Key :type "Key Structure"))
  (:`Pressed`
    (`/Engine/EditorBlueprintResources/StandardMacros.FlipFlop`
      (:`A`
        (`WidgetBlueprintLibrary.SetInputMode_GameAndUIEx` self (`self.WB_PauseMenu`))
        (set `self.bShowMouseCursor` true))
      (:`B`
        (`WidgetBlueprintLibrary.SetInputMode_GameOnly` self)
        (set `self.bShowMouseCursor` false)))))

(fn `UserConstructionScript`)